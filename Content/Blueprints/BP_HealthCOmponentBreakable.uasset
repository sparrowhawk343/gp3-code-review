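; Health component for breakable objects that turns damage taken into damage or destruction of its owning BP_BreakableBase.
; On damage, it calls DamageObject on the owner while health is above one, otherwise DestroyObject if still alive.
; Both outcomes first run SpawnFloaters, which shows floating text on a random one-in-three chance.
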(event EventOnDamageTaken
  (params (FromActor :type Actor%20Object%20Reference))
  (bind _asbp_breakable_base (Utilities|Casting|CastToBP_BreakableBase (Components|GetOwner)))
  (if (> (Variables|Default|GetCurrentHealth) 1)
    (CallFunction|SpawnFloaters)
    (Default|DamageObject _asbp_breakable_base)
    (elif (Variables|Default|GetIsAlive)
      (CallFunction|SpawnFloaters)
      (Default|DestroyObject _asbp_breakable_base))))

(fn SpawnFloaters
  (if (== (Class|KismetMathLibrary|RandomInteger64inRange 0 2) 0)
    (Class|HealthComponent|SpawnFloatingText)))