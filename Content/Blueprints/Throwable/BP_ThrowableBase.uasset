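; Base throwable actor that damages what it strikes and destroys itself on impact.
; The static mesh hit event acts only while the PickupComponent reports it is being thrown.
; If the hit actor has a HealthComponent, it takes damage through that component.
; Every thrown impact, damaging or not, spawns a scaled-down effect system at the actor's location before destroying it.
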(event OnComponentHit(StaticMeshComponent)
  (params (HitComponent :type Primitive%20Component%20Object%20Reference) (OtherActor :type Actor%20Object%20Reference) (OtherComp :type Primitive%20Component%20Object%20Reference) (NormalImpulse :type Vector :default "0, 0, 0") (Hit :type Hit%20Result%20Structure%20%28by%20ref%29))
  (bind _returnvalue (Actor|GetComponentbyClass OtherActor "/Script/Team05.HealthComponent"))
  (if (Variables|/Script/Team05.AC_Pickup|GetBeingThrown (Variables|Default|GetPickupComponent))
    (Utilities|IsValid _returnvalue
      (:Is%20Valid
        (Variables|Default|SetOtherHealthComponent _returnvalue)
        (Utilities|FlowControl|Sequence
          (:then_0
            (Class|HealthComponent|TakeDamage (Variables|Default|GetOtherHealthComponent) (Variables|/Script/Team05.HealthComponent|GetDamage (Variables|Default|GetHealth))))
          (:then_1
            (Niagara|SpawnSystematLocation "/Game/VFX/HalldorTestVFX/Test1_System_2.Test1_System_2" (Transformation|GetActorLocation) "0, 0, 0" "0.600000,0.600000,0.600000")
            (Actor|DestroyActor))))
      (:Is%20Not%20Valid
        (Niagara|SpawnSystematLocation "/Game/VFX/HalldorTestVFX/Test1_System_2.Test1_System_2" (Transformation|GetActorLocation) "0, 0, 0" "0.600000,0.600000,0.600000")
        (Actor|DestroyActor)))))

(fn ConstructionScript)