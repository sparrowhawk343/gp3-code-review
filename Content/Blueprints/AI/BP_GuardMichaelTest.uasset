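; Test guard AI character that roams or patrols, then approaches and shoots the player on sight.
; BeginPlay spawns its controller and picks behavior from AIState, using recursive AIMoveTo loops for roaming and two-point patrol.
; PawnSensing drives approach and montage-notify projectile fire with FMOD audio and a cooldown, while AIPerception sight only turns the guard.
; Tick and DamageAI are empty, leaving persistent-chase and hit/damage logic disconnected.
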(event OnTargetPerceptionUpdated(AIPerception)
  (params (Actor :type Actor%20Object%20Reference) (Stimulus :type AI%20Stimulus%20Structure))
  (bind _asbp_third_person_character (Utilities|Casting|CastToBP_ThirdPersonCharacter Actor))
  (bind _returnvalue (Class|AIPerceptionSystem|GetSenseClassforStimulus Stimulus))
  (switch string (Utilities|GetClassDisplayName _returnvalue)
    (:AiSense_Sight
      (Transformation|SetActorRotation (Math|Rotator|FindLookatRotation (Transformation|GetActorLocation) (Transformation|GetActorLocation _asbp_third_person_character))))))

(event OnSeePawn(PawnSensing)
  (params (Pawn :type Pawn%20Object%20Reference))
  ;[0.2299 1 0.7036] On sensing the player chase/shoot
  (bind _asbp_third_person_character (Utilities|Casting|CastToBP_ThirdPersonCharacter Pawn))
  (Utilities|FlowControl|Sequence
    (:then_0
      (Transformation|SetActorRotation (Math|Rotator|FindLookatRotation (Transformation|GetActorLocation) (Transformation|GetActorLocation _asbp_third_person_character)))
      (AI|AIMoveTo self "0, 0, 0" _asbp_third_person_character (Variables|Default|GetShootingRange) false))
    (:then_1
      (if (Variables|Default|GetbShootDelay)
        (if (not (Animation|Montage|MontageIsPlaying (Components|SkeletalMesh|GetAnimInstance (Variables|Character|GetMesh)) "/Game/Playercharacter/Animation/Monkey_Custom_Anim/Police_AttackTemp_Montage.Police_AttackTemp_Montage"))
          (Animation|Montage|PlayMontage (Variables|Character|GetMesh) "/Game/Playercharacter/Animation/Monkey_Custom_Anim/Police_AttackTemp_Montage.Police_AttackTemp_Montage" 3.0
            (:OnCompleted
              (Variables|Default|SetbShootDelay false)
              (Utilities|FlowControl|Delay (Variables|Default|GetShootTimer))
              (Variables|Default|SetbShootDelay true))
            (:OnNotifyBegin
              (CallFunction|ShootProjectile)
              (Class|FMODBlueprintStatics|PlayEventatLocation (Variables|Default|GetOnShootFMODEvent) (Math|Conversions|ToTransform(Vector) (Transformation|GetActorLocation))))))))
    (:then_2
      (Variables|Default|SetbHasSeenThePlayer true))))

(event Custom|RoamPoint
  ;[0.1043 0.1512 1] Roam For Move To Point
  (AI|AIMoveTo self (.RandomLocation (Class|NavigationSystemV1|GetRandomPointinNavigableRadius (Transformation|GetActorLocation) 7e+02 0 0)) 0 5e+01 false
    (:OnSuccess
      _)
    (:OnFail
      _))
  (Utilities|FlowControl|Delay 3.0)
  (CallFunction|RoamPoint))

(event Custom|ChasePlayer
  (params (PlayerToChase :type Pawn%20Object%20Reference))
  ;[1 0.2722 0.3821] Chase player
  (AI|AIMoveTo self "0, 0, 0" (Game|GetPlayerController 0) (Variables|Default|GetChaseRange) false))

(event Custom|Roam
  ;[1 0 0.7915] Roam within a radius
  (AI|AIMoveTo self (.RandomLocation (Class|NavigationSystemV1|GetRandomPointinNavigableRadius (Transformation|GetActorLocation) 1.5e+03 0 0)) 0 2e+02 false
    (:OnSuccess
      _)
    (:OnFail
      _))
  (Utilities|FlowControl|Delay 3.0)
  (CallFunction|Roam))

(event Custom|ShootProjectile
  ;[0.2299 1 0.7036] On sensing the player chase/shoot
  (Game|SpawnActorfromClass "/Game/Blueprints/AI/BP_Projectile.BP_Projectile_C" (Transformation|GetWorldTransform (Variables|Default|GetScene)) "Undefined" 0 0))

(event Custom|MoveToPointAndRoam
  ;[0.04231 0.06125 0.4072] MoveToPointAndRoam
  (bind _returnvalue (Actor|GetActorOfClass (Variables|Default|GetPatrollingPoint)))
  (AI|AIMoveTo self "0, 0, 0" _returnvalue 75.0 false
    (:OnSuccess
      (if (>= (Variables|Default|GetPatrolPointIndex) (- (Utilities|Array|Length (Variables|Default|GetPatrolPoints)) 1))
        (Variables|Default|SetPatrolPointIndex 0)
        (CallFunction|RoamPoint)
        (else
          (Math|Integer|IncrementInt (Variables|Default|GetPatrolPointIndex)))))))

(event Custom|PatrolPointToPoint
  ;[0.2657 1 0.286] Patrol
  (bind _output_get (Variables|Default|SetPatrolPoints (Utilities|Array|MakeArray (Variables|Default|GetPatrollingPoint1) (Variables|Default|GetPatrollingPoint2))))
  (bind _returnvalue (Actor|GetActorOfClass (Utilities|Array|Get(acopy) _output_get (Variables|Default|GetPatrolPointIndex))))
  (AI|AIMoveTo self "0, 0, 0" _returnvalue 1e+02 false
    (:OnSuccess
      (if (>= (Variables|Default|GetPatrolPointIndex) (- (Utilities|Array|Length (Variables|Default|GetPatrolPoints)) 1))
        (Variables|Default|SetPatrolPointIndex 0)
        (else
          (Math|Integer|IncrementInt (Variables|Default|GetPatrolPointIndex)
            (:%20%20
              _))))
      (Utilities|FlowControl|Delay 1.5)
      (CallFunction|PatrolPointtoPoint))))

(event EventTick
  (params (DeltaSeconds :type Float%20%28single-precision%29))
  ;[1 1 1] If seen the player chase him forever (Temp fix for the bug where you could get the AI stucked by walking in to them).
)

(event EventDamageAI
  (params (Actor :type Actor%20Object%20Reference))
  ;[1 0.9309 0.1014] GetHitAI
)

(event EventBeginPlay
  ;[1 1 1] Behavier setting / controller spawner
  (Utilities|FlowControl|Sequence
    (:then_0
      (Pawn|SpawnDefaultController))
    (:then_1
      (switch Utilities|FlowControl|Switch|SwitchonEnum_AIState (Variables|Default|GetAIState)
        (:NewEnumerator0
          (CallFunction|MovetoPointandRoam))
        (:NewEnumerator1
          (CallFunction|Roam))
        (:NewEnumerator2
          (CallFunction|ChasePlayer))
        (:NewEnumerator3
          (CallFunction|MovetoPointandRoam))
        (:NewEnumerator4
          (CallFunction|PatrolPointtoPoint))))))

(fn ConstructionScript)