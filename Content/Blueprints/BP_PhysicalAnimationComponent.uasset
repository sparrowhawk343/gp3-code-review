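; Actor component that gives its owning Character physics-driven hit reactions and death ragdolls, adding a PhysicalAnimation component for the mesh at BeginPlay.
; HitReaction simulates bodies from the Spine down with a profile, shoves the Head along the hit direction and starts a Tick countdown.
; Tick fades physics blend weight with remaining time, then restores the mesh and stops ticking.
; DeathRagDoll simulates the whole body with a stronger head impulse.
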(event Custom|TogglePhysicalAnimation)

(event Custom|HitReaction
  (params (HitDirection :type Vector))
  (bind _returnvalue (Utilities|Name|MakeLiteralName "Spine"))
  (bind _mesh (Variables|Default|GetMesh))
  ;[0.3333 1 1] HitReaction
  (Components|Tick|SetComponentTickEnabled true)
  (Variables|Default|SetTimeRemaining (+ 0.4 (Variables|Default|GetTimeRemaining)))
  (Class|PhysicalAnimationComponent|ApplyPhysicalAnimationProfileBelow (Variables|Default|GetPhysicalAnimationComponent) _returnvalue "HitReactionProfile" false false)
  (Class|SkeletalMeshComponent|SetAllBodiesBelowSimulatePhysics _mesh _returnvalue true true)
  (Collision|SetCollisionEnabled _mesh "PhysicsOnly")
  (Physics|AddImpulse _mesh (* HitDirection 4e+03) (Utilities|Name|MakeLiteralName "Head") false))

(event Custom|OnTickEnd
  (bind _mesh (Variables|Default|GetMesh))
  ;[1 1 1] Tick countdown
  (Collision|SetCollisionEnabled _mesh "NoCollision")
  (Class|SkeletalMeshComponent|ResetAllBodiesSimulatePhysics _mesh))

(event Custom|DeathRagDoll
  (params (HitDirection :type Vector))
  (bind _mesh (Variables|Default|GetMesh))
  ;[1 0.4762 0.6277] DeathRagdoll
  (Class|PhysicalAnimationComponent|ApplyPhysicalAnimationProfileBelow (Variables|Default|GetPhysicalAnimationComponent) (Utilities|Name|MakeLiteralName "Hips") "HitReactionProfile" true false)
  (Class|SkeletalMeshComponent|SetAllBodiesSimulatePhysics _mesh true)
  (Collision|SetCollisionEnabled _mesh "PhysicsOnly")
  (Physics|AddImpulse _mesh (* HitDirection 5e+03) (Utilities|Name|MakeLiteralName "Head") false))

(event EventBeginPlay
  (bind _returnvalue (Game|AddComponentbyClass (Components|GetOwner) "/Script/Engine.PhysicalAnimationComponent"))
  (bind _output_get (Variables|Default|SetPhysicalAnimationComponent _returnvalue))
  (bind _ascharacter (Utilities|Casting|CastToCharacter (Components|GetOwner)))
  (Class|PhysicalAnimationComponent|SetSkeletalMeshComponent _output_get (Variables|/Script/Engine.Character|GetMesh _ascharacter))
  (Variables|Default|SetMesh (Variables|/Script/Engine.Character|GetMesh _ascharacter)))

(event EventTick
  (params (DeltaSeconds :type Float%20%28single-precision%29))
  ;[1 1 1] Tick countdown
  (bind _output_get (Variables|Default|SetTimeRemaining (- (Math|Interpolation|FInterpTo (Variables|Default|GetTimeRemaining) 0.0 0.0 1.0) DeltaSeconds)))
  (if (<= _output_get 0.0)
    (Variables|Default|SetTimeRemaining 0.0)
    (Class|SkeletalMeshComponent|SetAllBodiesBelowSimulatePhysics (Variables|Default|GetMesh) (Utilities|Name|MakeLiteralName "Spine") false true)
    (Components|Tick|SetComponentTickEnabled false)
    (CallFunction|OnTickEnd)
    (else
      (Class|SkeletalMeshComponent|SetAllBodiesBelowPhysicsBlendWeight (Variables|Default|GetMesh) (Utilities|Name|MakeLiteralName "Spine") (Math|Float|Min(Float) (Variables|Default|GetTimeRemaining) 1.0) false true))))