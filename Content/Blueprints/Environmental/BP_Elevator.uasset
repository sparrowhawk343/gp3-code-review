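; Elevator actor whose doors unlock and open once the chaos meter reaches a set percentage, checked every Tick.
; Interacting closes the doors and broadcasts entry; the player leaving its collider broadcasts exit, closes them and re-arms the chaos check.
; One timeline plays forward or in reverse to slide both doors.
; When it finishes with the level-event flag set, it broadcasts closed or opened, setting the police timer on close.
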(event OnComponentEndOverlap(PlayerLeftCollider)
  (params (OverlappedComponent :type Primitive%20Component%20Object%20Reference) (OtherActor :type Actor%20Object%20Reference) (OtherComp :type Primitive%20Component%20Object%20Reference) (OtherBodyIndex :type Integer))
  (if (== OtherActor (Game|Player|GetPlayerPawn 0))
    (Default|CallOnElevatorExited)
    (Utilities|FlowControl|Sequence
      (:then_0
        (Variables|Default|SetCallEventInLevel false))
      (:then_1
        (Variables|Default|SetCanOpen true))
      (:then_2
        (CallFunction|CloseElevatorDoor))
      (:then_3
        (Class|FMODBlueprintStatics|PlayEventatLocation "/Game/FMOD/Events/Objects___Interactables/ElevatorClose.ElevatorClose" (Math|Conversions|ToTransform(Vector) (Transformation|GetActorLocation)))))))

(event Custom|OpenElevatorDoor
  (Utilities|FlowControl|Sequence
    (:then_0
      (Class|FMODBlueprintStatics|PlayEventatLocation "/Game/FMOD/Events/Objects___Interactables/ElevatorOpen.ElevatorOpen" (Transformation|GetActorTransform)))
    (:then_1
      (bind (_direction _closing) (Timeline|Elevator ReverseFromEnd)
        (:Update
          (CallFunction|UpdateElevatorDoors _closing))
        (:Finished
          (CallFunction|OnElevatorFinished _direction))))))

(event Custom|CloseElevatorDoor
  (Utilities|FlowControl|Sequence
    (:then_0
      (Class|FMODBlueprintStatics|PlayEventatLocation "/Game/FMOD/Events/Objects___Interactables/ElevatorClose.ElevatorClose" (Transformation|GetActorTransform)))
    (:then_1
      (bind (_direction _closing) (Timeline|Elevator PlayFromStart)
        (:Update
          (CallFunction|UpdateElevatorDoors _closing))
        (:Finished
          (CallFunction|OnElevatorFinished _direction))))))

(event Custom|ElevatorOpened
  (Default|CallOnElevatorOpened))

(event Custom|ElevatorClosed
  (Default|CallOnElevatorClosed))

(event Custom|UnlockElevator
  (CallFunction|OpenElevatorDoor))

(event EventInteract
  (if (Variables|Default|GetIs%20Interactible)
    (Utilities|FlowControl|Sequence
      (:then_0
        (Variables|Default|SetCallEventInLevel true))
      (:then_1
        (Variables|Default|SetIs%20Interactible false))
      (:then_2
        (CallFunction|CloseElevatorDoor))
      (:then_3
        (Default|CallOnElevatorEntered)))))

(event EventTick
  (params (DeltaSeconds :type Float%20%28single-precision%29))
  (if (and (CallFunction|DestroyedEnoughItems) (Variables|Default|GetCanOpen))
    (Utilities|FlowControl|Sequence
      (:then_0
        (Variables|Default|SetCallEventInLevel false))
      (:then_1
        (Variables|Default|SetCanOpen false))
      (:then_2
        (Variables|Default|SetIs%20Interactible true))
      (:then_3
        (CallFunction|OpenElevatorDoor))
      (:then_4
        (Class|FMODBlueprintStatics|PlayEventatLocation "/Game/FMOD/Events/Objects___Interactables/ElevatorUnlock.ElevatorUnlock" (Math|Conversions|ToTransform(Vector) (Transformation|GetActorLocation)))))))

(fn ConstructionScript)

(fn CheckifPlayerHasWalkedOverBothTriggers
  (if (Math|Boolean|Equal(Boolean) false false)
    (CallFunction|ElevatorOpened)))

(fn DestroyedEnoughItems
  (return (>= (Class|ChaosCounterAsset|GetPercent (Variables|Default|GetChaosMeter)) (/ (Variables|Default|GetElevator%20Open%20Procentage) 1e+02))))

(fn UpdateElevatorDoors
  (params (Alpha :type Float%20%28single-precision%29))
  (bind _returnvalue (Math|Float|Lerp 1.4e+02 0.0 Alpha))
  (bind _door1 (Variables|Default|GetDoor1))
  (bind _door2 (Variables|Default|GetDoor2))
  (bind _relativelocation (Variables|/Script/Engine.SceneComponent|GetRelativeLocation _door1))
  (bind _relativelocation_2 (Variables|/Script/Engine.SceneComponent|GetRelativeLocation _door2))
  (Utilities|FlowControl|Sequence
    (:then_0
      (Transformation|SetRelativeLocation _door1 (Math|Vector|MakeVector _returnvalue (.y _relativelocation) (.z _relativelocation)) false false))
    (:then_1
      (Transformation|SetRelativeLocation _door2 (Math|Vector|MakeVector (* _returnvalue -1.0) (.y _relativelocation_2) (.z _relativelocation_2)) false false))))

(fn OnElevatorFinished
  (params (Selection :type ETimelineDirection%20Enum :default "Forward"))
  (if (Variables|Default|GetCallEventInLevel)
    (switch Utilities|FlowControl|Switch|SwitchonETimelineDirection Selection
      (:Forward
        (CallFunction|ElevatorClosed)
        (Variables|/Script/Team05.PoliceTimerAsset|SetCurrentTimer (Variables|Default|GetPolice%20Timer%20Asset) 99.0))
      (:Backward
        (CallFunction|ElevatorOpened)
        (Variables|Default|SetCanOpen true)))))