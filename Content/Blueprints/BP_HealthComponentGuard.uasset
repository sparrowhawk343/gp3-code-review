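; BP_HealthComponentGuard is a health component for guards that responds when its owner takes damage.
; At zero health it triggers a death ragdoll on the owner's physical animation component and calls GuardDeath on BP_GuardBase.
; Otherwise it plays a physical hit reaction, makes the guard chase the player and plays a police hurt sound event at the guard's location.
; Both physical reactions take their direction from the attacker's forward vector.
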(event EventBeginPlay
  (|CallParentFunction) ; This node is disabled and will not be called.\nDrag off pins to build functionality.
)

(event EventTick
  (params (DeltaSeconds :type Float%20%28single-precision%29))
  (|CallParentFunction DeltaSeconds) ; This node is disabled and will not be called.\nDrag off pins to build functionality.
)

(event EventOnDamageTaken
  (params (FromActor :type Actor%20Object%20Reference))
  (bind _returnvalue (Components|GetOwner))
  (bind _returnvalue_2 (Components|GetOwner))
  (bind _returnvalue_3 (Actor|GetComponentbyClass _returnvalue_2 "/Game/Blueprints/BP_PhysicalAnimationComponent.BP_PhysicalAnimationComponent_C"))
  (Variables|Default|SetFrom%20Actor FromActor)
  (if (<= (Variables|Default|GetCurrentHealth) 0)
    (Default|DeathRagDoll (Actor|GetComponentbyClass _returnvalue "/Game/Blueprints/BP_PhysicalAnimationComponent.BP_PhysicalAnimationComponent_C") (Transformation|GetActorForwardVector (Variables|Default|GetFrom%20Actor)))
    (bind _asbp_guard_base (Utilities|Casting|CastToBP_GuardBase _returnvalue))
    (Default|GuardDeath _asbp_guard_base)
    (else
      (Utilities|FlowControl|Sequence
        (:then_0
          (Utilities|IsValid _returnvalue_3
            (:Is%20Valid
              (Default|HitReaction _returnvalue_3 (Transformation|GetActorForwardVector FromActor)))))
        (:then_1
          (bind _asbp_guard_base_2 (Utilities|Casting|CastToBP_GuardBase (Components|GetOwner)))
          (Default|ChasePlayer _asbp_guard_base_2))
        (:then_2
          (Class|FMODBlueprintStatics|PlayEventatLocation "/Game/FMOD/Events/Npc_s___Enemies/Police_Hurt.Police_Hurt" (Math|Conversions|ToTransform(Vector) (Transformation|GetActorLocation (Components|GetOwner)))))))))