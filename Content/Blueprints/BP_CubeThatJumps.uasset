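; BP_CubeThatJumps is a breakable object built from twelve cube components that bursts upward when reacted to.
; BeginPlay turns physics off on every cube so the object holds still.
; The first Inreact event spawns a particle effect, enables physics on each cube, applies an upward impulse, then sets IsDestroyed to block repeats.
; A pass switching the cubes' collision to ignore pawns is present but never runs.
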(event EventBeginPlay
  (for _array_element (Utilities|Array|MakeArray (Variables|Default|GetCube) (Variables|Default|GetCube1) (Variables|Default|GetCube2) (Variables|Default|GetCube3) (Variables|Default|GetCube4) (Variables|Default|GetCube5) (Variables|Default|GetCube6) (Variables|Default|GetCube7) (Variables|Default|GetCube8) (Variables|Default|GetCube9) (Variables|Default|GetCube10) (Variables|Default|GetCube11))
    (bind _asmesh_component (Utilities|Casting|CastToMeshComponent _array_element))
    (Physics|SetSimulatePhysics _asmesh_component false)))

(event EventInreact
  (if (not (Variables|Default|GetisDestroyed))
    (bind _returnvalue (AddComponent|AddParticleSystemComponent false))
    (Transformation|SetWorldScale3D _returnvalue "1.000000,1.000000,1.000000")
    (Utilities|FlowControl|Sequence
      (:then_0
        ;[1 1 1] Break object
        (for _array_element (Utilities|Array|MakeArray (Variables|Default|GetCube) (Variables|Default|GetCube1) (Variables|Default|GetCube2) (Variables|Default|GetCube3) (Variables|Default|GetCube4) (Variables|Default|GetCube5) (Variables|Default|GetCube6) (Variables|Default|GetCube7) (Variables|Default|GetCube8) (Variables|Default|GetCube9) (Variables|Default|GetCube10) (Variables|Default|GetCube11))
          (bind _asmesh_component (Utilities|Casting|CastToMeshComponent _array_element))
          (Physics|SetSimulatePhysics _asmesh_component true)
          (Physics|AddImpulse _asmesh_component (* (Math|Vector|VectorUp) 2e+04) "None" false))
        (Variables|Default|SetisDestroyed true)))))

(event EventTick
  (params (DeltaSeconds :type Float%20%28single-precision%29)))

(fn ConstructionScript)