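; GM_MasterLevel is a game mode Blueprint that provides player-side setup for the master level.
; Its Spawn function applies the VSync setting, spawns a BP_PlayerCamera, has player 0's HUD_Player create the player HUD, then returns the camera.
; Despite its name, VSyncOn turns VSync off and applies the user settings.
; No graph in the file calls Spawn.
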(fn ConstructionScript)

(fn Spawn
  (CallFunction|VSyncon)
  (bind _returnvalue (Game|SpawnActorfromClass "/Game/Blueprints/BP_PlayerCamera.BP_PlayerCamera_C" (Math|Transform|MakeTransform "0, 0, 0" "0, 0, 0" "1,1,1") "AlwaysSpawn" 0 0))
  (bind _ashud_player (Utilities|Casting|CastToHUD_Player (HUD|GetHUD (Game|GetPlayerController 0))))
  (Default|CreatePlayerHud _ashud_player)
  (return _returnvalue))

(fn VSyncon
  (bind _returnvalue (Settings|GetGameUserSettings))
  (Class|GameUserSettings|SetVSyncEnabled _returnvalue false)
  (Class|GameUserSettings|ApplySettings _returnvalue true))