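; Player camera actor that follows BP_ThirdPersonCharacter from a fixed base rotation and distance, with built-in screen shake.
; BeginPlay finds the player, snaps behind it along the camera's forward axis and caches the component's default rotation.
; Each Tick lerps toward that offset position for smooth follow, then applies shake.
; AddCameraShake adds clamped trauma, which decays over time and is squared to scale random rotational jitter around the default.
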(event Custom|AddCameraShake
  (params (add :type Float%20%28single-precision%29))
  (Variables|Default|Settrauma (Math|Float|Clamp(Float) (+ add (Variables|Default|Gettrauma)))))

(event EventBeginPlay
  (Utilities|FlowControl|Sequence
    (:then_0
      (bind _returnvalue (Actor|GetActorOfClass "/Game/Blueprints/BP_ThirdPersonCharacter.BP_ThirdPersonCharacter_C"))
      (Variables|Default|SetPlayer _returnvalue))
    (:then_1
      (Transformation|SetActorLocation (Transformation|GetActorLocation (Variables|Default|GetPlayer)) false true))
    (:then_2
      (Transformation|SetActorRotation (Variables|Default|GetCameraBaseRotation)))
    (:then_3
      (Transformation|SetActorLocation (+ (Transformation|GetActorLocation (Variables|Default|GetPlayer)) (* (Transformation|GetActorForwardVector) (* (Variables|Default|GetCameraDistance) -1.0))) false true))
    (:then_4
      (Variables|Default|SetDefaultRot (Variables|/Script/Engine.SceneComponent|GetRelativeRotation (Variables|CameraActor|GetCameraComponent))))))

(event EventTick
  (params (DeltaSeconds :type Float%20%28single-precision%29))
  (Utilities|FlowControl|Sequence
    (:then_0
      (CallFunction|UpdatePlayerCamera DeltaSeconds))
    (:then_1
      (CallFunction|PerformCameraShake DeltaSeconds))))

(fn ConstructionScript)

(fn UpdatePlayerCamera
  (params (delta :type Float%20%28single-precision%29))
  (Transformation|SetActorLocation (Math|Vector|Lerp(Vector) (Transformation|GetActorLocation) (+ (Transformation|GetActorLocation (Variables|Default|GetPlayer)) (* (Transformation|GetActorForwardVector) (* (Variables|Default|GetCameraDistance) -1.0))) (* delta (Variables|Default|GetCameraSmoothSpeed))) false true))

(fn PerformCameraShake
  (params (Deltatime :type Float%20%28single-precision%29))
  (bind _defaultrot (Variables|Default|GetDefaultRot))
  (bind _output_get (Variables|Default|Settrauma (Math|Float|Clamp(Float) (- (Variables|Default|Gettrauma) Deltatime))))
  (Variables|Default|SetcameraShake (Math|Float|Square _output_get))
  (Transformation|SetRelativeRotation (Variables|CameraActor|GetCameraComponent) (Math|Rotator|MakeRotator (+ (CallFunction|RandomShakeOffset) (.roll _defaultrot)) (+ (CallFunction|RandomShakeOffset) (.pitch _defaultrot)) (+ (CallFunction|RandomShakeOffset) (.yaw _defaultrot))) false false))

(fn RandomShakeOffset
  (return (* 5.0 (Variables|Default|GetcameraShake) (Math|Random|RandomFloatinRange -1.0 1.0))))