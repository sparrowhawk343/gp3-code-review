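; BP_TempBreakable is a simple, apparently placeholder, breakable actor that disappears with effects when broken.
; On BeginPlay it binds to the breaking delegate on Breakable, which triggers BreakObjectBP.
; Guarded by IsDestroyed to run once, that function hides the root and cube, disables collision, adds a particle system and plays the FMOD break event at its location.
; The actor is hidden rather than destroyed.
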(event Custom|BreakingObjectDelegate_Event_0
  (CallFunction|BreakObjectBP))

(event EventBeginPlay
  (EventDispatchers|AssignBreakingObjectDelegate (Variables|Default|GetBreakable) (delegate Custom|BreakingObjectDelegate_Event_0)))

(event Collision|EventActorBeginOverlap
  (params (OtherActor :type Actor%20Object%20Reference)))

(event EventTick
  (params (DeltaSeconds :type Float%20%28single-precision%29)))

(fn ConstructionScript)

(fn BreakObjectBP
  (if (not (Variables|Default|GetisDestroyed))
    (Utilities|FlowControl|Sequence
      (:then_0
        (Rendering|SetVisibility (Variables|Default|GetDefaultSceneRoot) false false)
        (Collision|SetActorEnableCollision false))
      (:then_1
        (AddComponent|AddParticleSystemComponent false)
        (Variables|Default|SetisDestroyed true))
      (:then_2
        (Class|FMODBlueprintStatics|PlayEventatLocation (Variables|Default|GetOnBreakFMODEvent) (Math|Conversions|ToTransform(Vector) (Transformation|GetActorLocation)))))))