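; BP_Player is a player with world-axis movement input that renders its surrounding line-of-sight area into a render target.
; Every tick it writes its location to the M_VisionConePlayerPos material parameter collection and clears VisionConeTarget.
; It line-traces the Visibility channel in half-degree steps around a full circle, pushing each endpoint slightly outward.
; The endpoints become a triangle fan around a fixed canvas center, drawn into that target as a visibility mask.
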(event EventTick
  (params (DeltaSeconds :type Float%20%28single-precision%29))
  (CallFunction|VisionConeSystem))

(event Input|AxisEvents|InputAxisMoveForward
  (params (AxisValue :type Float%20%28single-precision%29))
  (Pawn|Input|AddMovementInput "90.000000, 0, 0" AxisValue false))

(event Input|AxisEvents|InputAxisMoveRight
  (params (AxisValue :type Float%20%28single-precision%29))
  (Pawn|Input|AddMovementInput "0,90.000000, 0" AxisValue false))

(fn ConstructionScript)

(fn GenerateVisionCone
  (bind _returnvalue (Transformation|GetActorLocation))
  (bind _traceends (LocalVariables|GetTraceEnds))
  (Utilities|Array|Clear (LocalVariables|GetTraceEnds))
  (for _index (range 0 720)
    (bind (_outhit _returnvalue_2) (Collision|LineTraceByChannel _returnvalue (+ _returnvalue (* (Math|Vector|RotateVector (Transformation|GetActorForwardVector) (Math|Rotator|MakeRotator 0.0 0.0 (* _index 0.5))) (Variables|Default|GetTraceLength))) "TraceTypeQuery1" false 0 "None"))
    (if _returnvalue_2
      (Utilities|Array|Add _traceends (+ (.Location (Collision|BreakHitResult _outhit)) (* (Math|Vector|RotateVector (Transformation|GetActorForwardVector) (Math|Rotator|MakeRotator 0.0 0.0 (* _index 0.5))) 15.0)))
      (else
        (Utilities|Array|Add _traceends (+ (* (Math|Vector|RotateVector (Transformation|GetActorForwardVector) (Math|Rotator|MakeRotator 0.0 0.0 (* _index 0.5))) 15.0) (+ _returnvalue (* (Math|Vector|RotateVector (Transformation|GetActorForwardVector) (Math|Rotator|MakeRotator 0.0 0.0 (* _index 0.5))) (Variables|Default|GetTraceLength))))))))
  (return (LocalVariables|GetTraceEnds)))

(fn PrepareVisionConeTriangles
  (params (Trace%20Results :type Array%20of%20Vectors))
  (bind _returnvalue (Transformation|GetActorLocation))
  (bind _returnvalue_2 (Math|Vector|MakeVector 9e+02 9e+02 0.0))
  (Utilities|Array|Clear (Variables|Default|GetTriangles))
  (for _index (range 0 (- (Utilities|Array|Length Trace%20Results) 2))
    (Utilities|Array|Add (Variables|Default|GetTriangles) (Utilities|Struct|MakeCanvasUVTri (Math|Conversions|ToVector2D(Vector) _returnvalue_2) "(X=0.000000,Y=0.000000)" "(R=1.000000,G=1.000000,B=1.000000,A=0.000000)" (Math|Conversions|ToVector2D(Vector) (+ (- (Utilities|Array|Get(acopy) Trace%20Results _index) _returnvalue) _returnvalue_2)) "(X=0.000000,Y=0.000000)" "(R=1.000000,G=1.000000,B=1.000000,A=0.000000)" (Math|Conversions|ToVector2D(Vector) (+ (- (Utilities|Array|Get(acopy) Trace%20Results (+ _index 1)) _returnvalue) _returnvalue_2)) "(X=0.000000,Y=0.000000)" "(R=1.000000,G=1.000000,B=1.000000,A=0.000000)")))
  (return (Variables|Default|GetTriangles)))

(fn VisionConeSystem
  (Utilities|FlowControl|Sequence
    (:then_0
      (Rendering|Material|SetVectorParameterValue "/Game/Materials/PostProcessing/M_VisionConePlayerPos.M_VisionConePlayerPos" "PlayerPos" (Math|Conversions|ToLinearColor(Vector) (Transformation|GetActorLocation)) :!class /Script/Engine.KismetMaterialLibrary))
    (:then_1
      (Rendering|ClearRenderTarget2D (Variables|Default|GetVisionConeTarget))
      (bind (_canvas _size _context) (Rendering|BeginDrawCanvastoRenderTarget "/Game/Materials/PostProcessing/VisionConeTarget.VisionConeTarget"))
      (bind _trace_results (CallFunction|GenerateVisionCone))
      (bind _triangles (CallFunction|PrepareVisionConeTriangles _trace_results))
      (Class|Canvas|DrawTriangle _canvas 0 _triangles)
      (Rendering|EndDrawCanvastoRenderTarget _context))))